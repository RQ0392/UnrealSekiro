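; Base enemy character with health, a lock-on reticle, distance-based melee or other montage attacks, and death handling.
; Damage updates the health bar widget, then either plays a hit montage or stops AI logic, movement and montages at zero health.
; Attacks pick randomly among montages whose range fits the player's distance, then signal completion, delayed if interrupted.
; A separate event switches the mesh to ragdoll with a timed lifespan.
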(event Custom|Execute_Attack
  (bind _selectedmontage (CallFunction|GetBestAttack))
  (Animation|Montage|PlayMontage (Variables|Character|GetMesh) _selectedmontage
    (:OnCompleted
      _)
    (:OnInterrupted
      (Utilities|FlowControl|Delay 1.2)))
  (Default|CallAttackFinished))

(event Custom|EnableRagdoll
  (bind _mesh (Variables|Character|GetMesh))
  (Collision|SetCollisionEnabled (Variables|Collision|GetCapsuleComponent) "NoCollision")
  (Collision|SetCollisionEnabled _mesh "NoCollision")
  (Collision|SetCollisionProfileName _mesh "Ragdoll" true :!class /Script/Engine.PrimitiveComponent)
  (Class|SkeletalMeshComponent|SetAllBodiesSimulatePhysics (Variables|Character|GetMesh) true)
  (Actor|SetLifeSpan 4.0))

(event Custom|SetTargetedStatus_1
  (params (Status :type Boolean))
  (bind _lockonreticle (Variables|Default|GetLockOnreticle))
  ;[0.15 0.15 0.15 0.5] Lock
  (Development|PrintString "gOT")
  (bind _output_get (Variables|Default|SetIsTargeted Status))
  (if _output_get
    (Rendering|SetVisibility _lockonreticle true false)
    (else
      (Rendering|SetVisibility _lockonreticle false false))))

(event Game|Damage|EventAnyDamage
  (params (Damage :type Float%20%28single-precision%29) (DamageType :type Damage%20Type%20Object%20Reference) (InstigatedBy :type Controller%20Object%20Reference) (DamageCauser :type Actor%20Object%20Reference))
  (bind _charactermovement (Variables|Character|GetCharacterMovement))
  ;[0.15 0.15 0.15 0.5] EnemyHP and Anim
  (CallFunction|TakeRQDamage Damage "0, 0, 0" DamageCauser)
  (bind _aswbp_health_bar (Utilities|Casting|CastToWBP_HealthBar (UserInterface|GetUserWidgetObject (Variables|Default|GetHealthBar))))
  (Default|UpdateHealth _aswbp_health_bar (Variables|Default|GetCurrentHealth) (Variables|Default|GetMaxHealth))
  ;;[0.15 0.15 0.15 0.5] Disable actor capsule and trigger mesh physical simulation for death ragdoll
  (if (<= (Variables|Default|GetCurrentHealth) 0.0)
    (Variables|Default|SetIsDead true)
    (bind _asaicontroller (Utilities|Casting|CastToAIController (Pawn|GetController)))
    (AI|Logic|StopLogic (Variables|/Script/AIModule.AIController|GetBrainComponent _asaicontroller) "")
    (Components|Movement|StopMovementImmediately _charactermovement)
    (Pawn|Components|CharacterMovement|DisableMovement _charactermovement)
    (Animation|StopAnimMontage 0)
    (else
      (Animation|PlayAnimMontage (Variables|Default|GetHitMontage) 1.0 "None"))))

(event EventBeginPlay
  (Utilities|FlowControl|Sequence
    (:then_0
      (Variables|Default|SetIsDead false)
      (bind _output_get (Variables|Default|SetMaxHealth 1e+02))
      (Variables|Default|SetCurrentHealth _output_get))))

(event EventTakeRQDamage
  (params (DamageAmount :type Float%20%28double-precision%29) (HitLocation :type Vector :default "0, 0, 0") (Attacker :type Actor%20Object%20Reference))
  (bind _charactermovement (Variables|Character|GetCharacterMovement))
  ;[0.15 0.15 0.15 0.5] EnemyHP and Anim
  (if (not (Variables|Default|GetIsDead))
    (Variables|Default|SetCurrentHealth (Math|Float|Clamp(Float) (- (Variables|Default|GetCurrentHealth) DamageAmount) 0.0 (Variables|Default|GetMaxHealth)))
    (bind _aswbp_health_bar (Utilities|Casting|CastToWBP_HealthBar (UserInterface|GetUserWidgetObject (Variables|Default|GetHealthBar))))
    (Default|UpdateHealth _aswbp_health_bar (Variables|Default|GetCurrentHealth) (Variables|Default|GetMaxHealth))
    ;;[0.15 0.15 0.15 0.5] Disable actor capsule and trigger mesh physical simulation for death ragdoll
    (if (<= (Variables|Default|GetCurrentHealth) 0.0)
      (Variables|Default|SetIsDead true)
      (bind _asaicontroller (Utilities|Casting|CastToAIController (Pawn|GetController)))
      (AI|Logic|StopLogic (Variables|/Script/AIModule.AIController|GetBrainComponent _asaicontroller) "")
      (Components|Movement|StopMovementImmediately _charactermovement)
      (Pawn|Components|CharacterMovement|DisableMovement _charactermovement)
      (Animation|StopAnimMontage 0)
      (else
        (Animation|PlayAnimMontage (Variables|Default|GetHitMontage) 1.0 "None")))))

(fn ConstructionScript)

(fn GetBestAttack
  (bind _candidateattacks (Variables|Default|GetCandidateAttacks))
  (bind _asbp_rq_character (Utilities|Casting|CastToBP_RQ_Character (Game|GetPlayerCharacter 0)))
  (bind _output_get (Variables|Default|SetRefPlayerCharacter _asbp_rq_character))
  (Utilities|Array|Clear (Variables|Default|GetCandidateAttacks))
  (for _array_element (Variables|Default|GetAttackList)
    (if (and (>= (Transformation|GetDistanceTo _output_get) (.mindistance _array_element)) (<= (Transformation|GetDistanceTo _output_get) (.maxdistance _array_element)))
      (bind _returnvalue (Utilities|Array|Add _candidateattacks (.atkmontage _array_element)))))
  (return (Utilities|Array|Get(acopy) _candidateattacks (Math|Random|RandomIntegerinRange 0 (Math|Random|RandomInteger (Utilities|Array|Length _candidateattacks))))))