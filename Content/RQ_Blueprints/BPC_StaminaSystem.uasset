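; Stamina component that tracks a pool for sprinting and other costed actions.
; Each Tick it drains stamina while IsSprinting, otherwise regenerates it once a delay since the last sprint has passed.
; ConsumeStamina can push the value into a clamped negative debt, while HasEnoughStamina only passes above zero.
; Tick also prints current stamina for debugging, and the BeginPlay character cast leads to no logic.
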(event EventBeginPlay
  ;[0.15 0.15 0.15 0.5] Todelete
  (Utilities|Casting|CastToBP_RQ_Character (Variables|Default|GetCharacterRef)))

(event EventTick
  (params (DeltaSeconds :type Float%20%28single-precision%29))
  (Development|PrintString (Utilities|String|ToString(Float) (Variables|Default|GetCurrentStamina)))
  (if (Variables|Default|GetIsSprinting)
    (CallFunction|ConsumeStamina (* (Utilities|Time|GetWorldDeltaSeconds) (Variables|Default|GetSprintDrainRate)))
    (Variables|Default|SetTimeSinceLastConsume 0.0)
    (else
      (Variables|Default|SetTimeSinceLastConsume (+ (Variables|Default|GetTimeSinceLastConsume) (Utilities|Time|GetWorldDeltaSeconds)))
      (if (> (Variables|Default|GetTimeSinceLastConsume) (Variables|Default|GetRegenDelay))
        (Variables|Default|SetCurrentStamina (Math|Float|Clamp(Float) (+ (Variables|Default|GetCurrentStamina) (* (Variables|Default|GetStaminaRegenRate) (Utilities|Time|GetWorldDeltaSeconds))) -5e+01 (Variables|Default|GetMaxStamina)))))))

(fn HasEnoughStamina
  (return (> (Variables|Default|GetCurrentStamina) 0.0)))

(fn ConsumeStamina
  (params (CostAmount :type Float%20%28double-precision%29))
  (Variables|Default|SetCurrentStamina (Math|Float|Clamp(Float) (- (Variables|Default|GetCurrentStamina) CostAmount) -5e+01 (Variables|Default|GetMaxStamina))))