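; Souls-like player character with Enhanced Input movement, stamina-gated sprint, jumping, three-step montage combos and health with hit reactions and ragdoll death.
; Lock-on picks the enemy most aligned with the camera by dot product, then Tick turns controller and actor toward it.
; Tick also tracks speed and air time, passing air time to the AnimInstance on landing.
; Screen-space target switching and line-of-sight unlock are unfinished and disconnected.
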(event Custom|ExecuteAttack
  ;[0.15 0.15 0.15 0.5] Unified execution point: handles buffer clearing, state locking, and montage playback.
  (Variables|State|SetIsAttacking true)
  (Animation|Montage|PlayMontage (Variables|Character|GetMesh) (Utilities|Array|Get(acopy) (Variables|Animations|GetAttackMontage) (Variables|Animations|GetComboIndex))
    (:then
      (Variables|Animations|SetComboIndex (Math|Integer|%(Integer) (+ (Variables|Animations|GetComboIndex) 1) 3)))))

(event Input|EnhancedActionEvents|EnhancedInputActionIA_Move
  (params (ActionValue :type Vector%202D%20Structure) (ElapsedSeconds :type Float%20%28double-precision%29) (TriggeredSeconds :type Float%20%28double-precision%29) (InputAction :type Input%20Action%20Object%20Reference :default "/Game/RQ_Input/Actions/IA_Move.IA_Move"))
  (bind _returnvalue (Pawn|GetControlRotation :!class /Script/Engine.Pawn))
  (bind _yaw (Math|Rotator|BreakRotator _returnvalue))
  (bind _returnvalue_2 (Math|Rotator|MakeRotator 0.0 0.0 _yaw))
  ;[0.15 0.15 0.15 0.5] Souls-like Movement: Decouple Actor Rotation from Camera-Relative Direction
  (if (not (Variables|Character|GetbIsStunned))
    (Pawn|Input|AddMovementInput (Math|Vector|GetForwardVector _returnvalue_2) (.y ActionValue) false)
    (Pawn|Input|AddMovementInput (Math|Vector|GetRightVector _returnvalue_2) (.x ActionValue) false)))

(event Input|EnhancedActionEvents|EnhancedInputActionIA_Sprint
  (params (ActionValue :type Boolean) (ElapsedSeconds :type Float%20%28double-precision%29) (TriggeredSeconds :type Float%20%28double-precision%29) (InputAction :type Input%20Action%20Object%20Reference :default "/Game/RQ_Input/Actions/IA_Sprint.IA_Sprint"))
  (bind _bpc_staminasystem (Variables|Default|GetBPC_StaminaSystem))
  ;[0.15 0.15 0.15 0.5] Sprint
  (:Triggered
    (bind _isenough (Default|HasEnoughStamina (Variables|Default|GetBPC_StaminaSystem)))
    (if _isenough
      (Variables|Character|SetbIsSprinting true)
      (Variables|/Script/Engine.CharacterMovementComponent|SetMaxWalkSpeed (Variables|Character|GetCharacterMovement) 5.5e+02)
      (Variables|/Game/RQ_Blueprints/BPC_StaminaSystem.BPC_StaminaSystem_C|SetIsSprinting _bpc_staminasystem true)
      (Development|PrintString "Hello")
      (else
        (Variables|Character|SetbIsSprinting false :!label _label)
        (Variables|/Script/Engine.CharacterMovementComponent|SetMaxWalkSpeed (Variables|Character|GetCharacterMovement) 4e+02)
        (Variables|/Game/RQ_Blueprints/BPC_StaminaSystem.BPC_StaminaSystem_C|SetIsSprinting _bpc_staminasystem false))))
  (:Completed
    (goto _label)))

(event Input|EnhancedActionEvents|EnhancedInputActionIA_ConsoleLook
  (params (ActionValue :type Vector%202D%20Structure) (ElapsedSeconds :type Float%20%28double-precision%29) (TriggeredSeconds :type Float%20%28double-precision%29) (InputAction :type Input%20Action%20Object%20Reference :default "/Game/RQ_Input/Actions/IA_ConsoleLook.IA_ConsoleLook"))
  ;[0.15 0.15 0.15 0.5] Split 2D input into Yaw (Horizontal) and Pitch (Vertical) for camera control
  (CallFunction|HandleCameraLook (.x ActionValue) (.y ActionValue)))

(event Input|EnhancedActionEvents|EnhancedInputActionIA_MouseLook
  (params (ActionValue :type Vector%202D%20Structure) (ElapsedSeconds :type Float%20%28double-precision%29) (TriggeredSeconds :type Float%20%28double-precision%29) (InputAction :type Input%20Action%20Object%20Reference :default "/Game/RQ_Input/Actions/IA_MouseLook.IA_MouseLook"))
  ;[0.15 0.15 0.15 0.5] Split 2D input into Yaw (Horizontal) and Pitch (Vertical) for camera control
  (Utilities|IsValid (Variables|Combat|Targeting|GetCurrentLockedTarget)
    (:Is%20Not%20Valid
      (CallFunction|HandleCameraLook (.x ActionValue) (.y ActionValue)))))

(event Input|EnhancedActionEvents|EnhancedInputActionIA_Jump
  (params (ActionValue :type Boolean) (ElapsedSeconds :type Float%20%28double-precision%29) (TriggeredSeconds :type Float%20%28double-precision%29) (InputAction :type Input%20Action%20Object%20Reference :default "/Game/RQ_Input/Actions/IA_Jump.IA_Jump"))
  ;[0.15 0.15 0.15 0.5] Sprint
  (:Started
    (if (Variables|State|GetbCanJump)
      (Character|Jump))))

(event Input|EnhancedActionEvents|EnhancedInputActionIA_Target
  (params (ActionValue :type Boolean) (ElapsedSeconds :type Float%20%28double-precision%29) (TriggeredSeconds :type Float%20%28double-precision%29) (InputAction :type Input%20Action%20Object%20Reference :default "/Game/RQ_Input/Actions/IA_Target.IA_Target"))
  ;[0.15 0.15 0.15 0.5] Lock
  (:Started
    (Utilities|IsValid (Variables|Combat|Targeting|GetCurrentLockedTarget)
      (:Is%20Valid
        (Class|BPIRQTargetable|SetTargetedStatus(Message) (Variables|Combat|Targeting|GetCurrentLockedTarget) false) ; Unlock
        (Variables|Combat|Targeting|SetCurrentLockedTarget 0)
        (Variables|/Script/Engine.CharacterMovementComponent|SetbOrientRotationToMovement (Variables|Character|GetCharacterMovement) true))
      (:Is%20Not%20Valid
        (Variables|Combat|Targeting|SetBest%20Target 0)
        (Variables|Combat|Targeting|SetMaxDotProduct -1.0)
        (bind _outactors (Collision|SphereOverlapActors (Transformation|GetActorLocation) 1.5e+03 (Utilities|Array|MakeArray "ObjectTypeQuery3" "ObjectTypeQuery2") "/Game/RQ_Blueprints/BP_RQ_Enemy_Base.BP_RQ_Enemy_Base_C"))
        (Development|PrintString (Utilities|String|ToString(Integer) (Utilities|Array|Length _outactors)))
        (for _array_element _outactors
          (Class|BPIRQTargetable|IsTargetable?(Message) _array_element false)
          (Development|PrintString (Utilities|String|ToString(Float) (Math|Vector|DotProduct (Math|Vector|GetForwardVector (Variables|Components|GetCamera)) (Math|Vector|Normalize (- (Transformation|GetActorLocation _array_element) (Transformation|GetWorldLocation (Variables|Components|GetCamera)))))))
          (if (> (Math|Vector|DotProduct (Math|Vector|GetForwardVector (Variables|Components|GetCamera)) (Math|Vector|Normalize (- (Transformation|GetActorLocation _array_element) (Transformation|GetWorldLocation (Variables|Components|GetCamera))))) (Variables|Combat|Targeting|GetMaxDotProduct))
            (bind _asbp_rq_enemy_base (Utilities|Casting|CastToBP_RQ_Enemy_Base _array_element))
            (bind _output_get (Variables|Combat|Targeting|SetMaxDotProduct (Math|Vector|DotProduct (Math|Vector|GetForwardVector (Variables|Components|GetCamera)) (Math|Vector|Normalize (- (Transformation|GetActorLocation _array_element) (Transformation|GetWorldLocation (Variables|Components|GetCamera)))))))
            (if (> _output_get 0.1)
              (bind _output_get_2 (Variables|Combat|Targeting|SetBest%20Target _asbp_rq_enemy_base)))))
        (Utilities|IsValid (Variables|Combat|Targeting|GetBest%20Target)
          (:Is%20Valid
            (bind _output_get_3 (Variables|Combat|Targeting|SetCurrentLockedTarget _output_get_2))
            (Class|BPIRQTargetable|SetTargetedStatus(Message) _output_get_3 true)
            (Variables|/Script/Engine.CharacterMovementComponent|SetbOrientRotationToMovement (Variables|Character|GetCharacterMovement) true)
            (Development|PrintString (Utilities|GetDisplayName _output_get_3)))
          (:Is%20Not%20Valid
            (Development|PrintString "Not Valid")))))))

(event Input|EnhancedActionEvents|EnhancedInputActionIA_Attack01
  (params (ActionValue :type Boolean) (ElapsedSeconds :type Float%20%28double-precision%29) (TriggeredSeconds :type Float%20%28double-precision%29) (InputAction :type Input%20Action%20Object%20Reference :default "/Game/RQ_Input/Actions/IA_Attack01.IA_Attack01"))
  (:Started
    (if (Variables|State|GetIsAttacking)
      (if (Variables|State|GetbIsComboWindowOpen)
        (CallFunction|ExecuteAttack :!label _label))
      (else
        (goto _label)))))

(event EventTick
  (params (DeltaSeconds :type Float%20%28single-precision%29))
  (bind _returnvalue (Transformation|GetActorLocation))
  (bind _charactermovement (Variables|Character|GetCharacterMovement))
  (Utilities|FlowControl|Sequence
    (:then_0
      ;[0.15 0.15 0.15 0.5] Get acceleration, speed, in air time
      (Variables|Character|SetSpeed (Math|Vector|VectorLength (Transformation|GetVelocity (Components|GetOwner _charactermovement))))
      (Variables|Character|SetbIsAccelerating (> (Math|Vector|VectorLength (Pawn|Components|CharacterMovement|GetCurrentAcceleration _charactermovement)) 0.0))
      (Variables|Character|SetbIsInAir (AI|Components|NavMovement|IsFalling (Variables|Character|GetCharacterMovement)))
      (if (Variables|Character|GetbIsInAir)
        (Variables|Character|SetAirTime (+ DeltaSeconds (Variables|Character|GetAirTime)))))
    (:then_1
      ;[0.15 0.15 0.15 0.5] Set Control and Mesh After Locked
      (Utilities|IsValid (Variables|Combat|Targeting|GetCurrentLockedTarget)
        (:Is%20Valid
          (Pawn|SetControlRotation (Game|GetPlayerController 0) (Math|Rotator|MakeRotator 0.0 (Math|Float|Clamp(Float) (.pitch (CallFunction|CalculateSmoothLookatRotation _returnvalue (Transformation|GetActorLocation (Variables|Combat|Targeting|GetCurrentLockedTarget)) (Pawn|GetControlRotation :!class /Script/Engine.Pawn))) 0.0 0.0) (.yaw (CallFunction|CalculateSmoothLookatRotation _returnvalue (Transformation|GetActorLocation (Variables|Combat|Targeting|GetCurrentLockedTarget)) (Pawn|GetControlRotation :!class /Script/Engine.Pawn)))))
          (Transformation|SetActorRotation (Math|Rotator|MakeRotator 0.0 0.0 (.yaw (CallFunction|CalculateSmoothLookatRotation _returnvalue (Transformation|GetActorLocation (Variables|Combat|Targeting|GetCurrentLockedTarget)) (Transformation|GetActorRotation)))))
          ;[0.15 0.15 0.15 0.5] TODO!!!FIX AFTER
          (Utilities|CheckShouldUnlock
            (:Instant
              _)
            (:buffer
              _))
          (Class|BPIRQTargetable|SetTargetedStatus(Message) (Variables|Combat|Targeting|GetCurrentLockedTarget) false)
          (Variables|Combat|Targeting|SetCurrentLockedTarget 0)
          (Variables|/Script/Engine.CharacterMovementComponent|SetbOrientRotationToMovement (Variables|Character|GetCharacterMovement) true))))))

(event EventIResetCombo
  (Variables|State|SetIsAttacking false)
  (Variables|Animations|SetComboIndex 0))

(event EventOnLanded
  (params (Hit :type Hit%20Result%20Structure%20%28by%20ref%29))
  ;[0.15 0.15 0.15 0.5] transmit Heavyland Signal
  (Utilities|FlowControl|Sequence
    (:then_0
      (Class|BPIRQPlayerAnimSignals|OnHeavyLandSignal(Message) (Components|SkeletalMesh|GetAnimInstance (Variables|Character|GetMesh)) (.z (Variables|/Script/Engine.MovementComponent|GetVelocity (Variables|Character|GetCharacterMovement))) (Variables|Character|GetAirTime)))
    (:then_1
      (Utilities|FlowControl|Delay 0.2)
      (Variables|State|SetbCanJump true))))

(event EventBeginPlay
  ;[0.15 0.15 0.15 0.5] Initialize Enhanced Input & Mapping Context                                                                                      (Bootstrap: Register Enhanced Input Mapping Context on BeginPlay)
  (bind _output_get (Variables|Stats|SetMaxHealth 1e+02))
  (Variables|Stats|SetCurrentHealth _output_get)
  (Input|AddMappingContext (PlayerController|LocalPlayerSubsystems|GetEnhancedInputLocalPlayerSubsystem (Game|GetPlayerController 0)) "/Game/RQ_Input/IMC_Default.IMC_Default" 0 "(bIgnoreAllPressedKeysUntilRelease=True,bForceImmediately=False,bNotifyUserSettings=False)")
  (Variables|/Script/Engine.CharacterMovementComponent|SetMaxWalkSpeed (Variables|Character|GetCharacterMovement) 4e+02))

(event EventTakeRQDamage
  (params (DamageAmount :type Float%20%28double-precision%29) (HitLocation :type Vector :default "0, 0, 0") (Attacker :type Actor%20Object%20Reference))
  (bind _mesh (Variables|Character|GetMesh))
  ;[0.15 0.15 0.15 0.5] Character HP
  (Variables|Stats|SetCurrentHealth (Math|Float|Clamp(Float) (- (Variables|Stats|GetCurrentHealth) DamageAmount) 0.0 (Variables|Stats|GetMaxHealth)))
  (if (<= (Variables|Stats|GetCurrentHealth) 0.0)
    ;;[0.15 0.15 0.15 0.5] Disable actor capsule and trigger mesh physical simulation for death ragdoll
    (Collision|SetCollisionEnabled (Variables|Collision|GetCapsuleComponent) "NoCollision")
    (Animation|Montage|PlayMontage (Variables|Character|GetMesh) (Variables|Animations|GetDeathMontage)
      (:OnCompleted
        (Collision|SetCollisionProfileName _mesh "Ragdoll" true :!class /Script/Engine.PrimitiveComponent)
        (Physics|SetSimulatePhysics _mesh true)))
    (else
      (Animation|PlayAnimMontage (Variables|Animations|GetHitMontage) 1.0 "None"))))

(fn ConstructionScript)

(fn FindNextTarget
  (params (LockOnDirection :type E_RQ_LockOnDirection%20Enum :default "NewEnumerator0"))
  (Variables|Combat|Targeting|SetRef_ScreenPos (.ScreenPosition (Class|GameplayStatics|ProjectWorldtoScreen (Game|GetPlayerController 0) (Transformation|GetActorLocation (Variables|Combat|Targeting|GetCurrentLockedTarget)) false)))
  (Variables|Combat|Targeting|SetMinScore 9999.0)
  (bind _outactors (Actor|GetAllActorswithInterface "/Game/RQ_Blueprints/Framework/BPI_RQ_Targetable.BPI_RQ_Targetable_C"))
  (for _array_element _outactors
    (if (not (== _array_element (Variables|Combat|Targeting|GetCurrentLockedTarget))) ; OnlyLockIsNotLockedtarget
      (if (.ReturnValue (Class|GameplayStatics|ProjectWorldtoScreen (Game|GetPlayerController 0) (Transformation|GetActorLocation _array_element) false))
        (Variables|Combat|Targeting|SetCandidate_ScreenPos (.ScreenPosition (Class|GameplayStatics|ProjectWorldtoScreen (Game|GetPlayerController 0) (Transformation|GetActorLocation _array_element) false)))
        (if (and (> (* (Utilities|Select :Index LockOnDirection :NewEnumerator0 (.x (- (Variables|Combat|Targeting|GetCandidate_ScreenPos) (Variables|Combat|Targeting|GetRef_ScreenPos))) :NewEnumerator1 (.x (- (Variables|Combat|Targeting|GetCandidate_ScreenPos) (Variables|Combat|Targeting|GetRef_ScreenPos))) :NewEnumerator2 (.y (- (Variables|Combat|Targeting|GetCandidate_ScreenPos) (Variables|Combat|Targeting|GetRef_ScreenPos))) :NewEnumerator3 (.y (- (Variables|Combat|Targeting|GetCandidate_ScreenPos) (Variables|Combat|Targeting|GetRef_ScreenPos)))) (Utilities|Select :Index LockOnDirection :NewEnumerator0 -1.0 :NewEnumerator1 1.0 :NewEnumerator2 -1.0 :NewEnumerator3 1.0)) 0.0) (< (* (Utilities|Select :Index LockOnDirection :NewEnumerator0 (.x (- (Variables|Combat|Targeting|GetCandidate_ScreenPos) (Variables|Combat|Targeting|GetRef_ScreenPos))) :NewEnumerator1 (.x (- (Variables|Combat|Targeting|GetCandidate_ScreenPos) (Variables|Combat|Targeting|GetRef_ScreenPos))) :NewEnumerator2 (.y (- (Variables|Combat|Targeting|GetCandidate_ScreenPos) (Variables|Combat|Targeting|GetRef_ScreenPos))) :NewEnumerator3 (.y (- (Variables|Combat|Targeting|GetCandidate_ScreenPos) (Variables|Combat|Targeting|GetRef_ScreenPos)))) (Utilities|Select :Index LockOnDirection :NewEnumerator0 -1.0 :NewEnumerator1 1.0 :NewEnumerator2 -1.0 :NewEnumerator3 1.0)) (Variables|Combat|Targeting|GetMinScore)))
          (Variables|Combat|Targeting|SetMinScore (* (Utilities|Select :Index LockOnDirection :NewEnumerator0 (.x (- (Variables|Combat|Targeting|GetCandidate_ScreenPos) (Variables|Combat|Targeting|GetRef_ScreenPos))) :NewEnumerator1 (.x (- (Variables|Combat|Targeting|GetCandidate_ScreenPos) (Variables|Combat|Targeting|GetRef_ScreenPos))) :NewEnumerator2 (.y (- (Variables|Combat|Targeting|GetCandidate_ScreenPos) (Variables|Combat|Targeting|GetRef_ScreenPos))) :NewEnumerator3 (.y (- (Variables|Combat|Targeting|GetCandidate_ScreenPos) (Variables|Combat|Targeting|GetRef_ScreenPos)))) (Utilities|Select :Index LockOnDirection :NewEnumerator0 -1.0 :NewEnumerator1 1.0 :NewEnumerator2 -1.0 :NewEnumerator3 1.0)))
          (Variables|Combat|Targeting|SetBestCandidate _array_element)))))
  (Class|BPIRQTargetable|SetTargetedStatus(Message) (Variables|Combat|Targeting|GetCurrentLockedTarget) false)
  (Utilities|IsValid (Variables|Combat|Targeting|GetBestCandidate)
    (:Is%20Valid
      (Variables|Combat|Targeting|SetCurrentLockedTarget (Variables|Combat|Targeting|GetBestCandidate))
      (Class|BPIRQTargetable|SetTargetedStatus(Message) (Variables|Combat|Targeting|GetBestCandidate) true))))

(fn CalculateSmoothLookatRotation
  (params (Start :type Vector%20%28by%20ref%29) (Target :type Vector%20%28by%20ref%29) (CurrentRotation :type Rotator))
  (return (Math|Interpolation|RInterpTo (Math|Rotator|FindLookatRotation Start Target) CurrentRotation (Utilities|Time|GetWorldDeltaSeconds) 3e+01)))

(fn HandleCameraLook
  (params (X :type Float%20%28single-precision%29) (Y :type Float%20%28single-precision%29))
  (Pawn|Input|AddControllerYawInput X)
  (Pawn|Input|AddControllerPitchInput Y)
  (return))